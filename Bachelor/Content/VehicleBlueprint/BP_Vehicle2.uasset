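; Traffic car that drives along world Y, turns through three flagged stages toward GameState points, then continues along X.
; Run_Event adds a random GameState mesh and body color.
; Tick moves it by swept transforms, slowing for the Stops flag, freezing behind another BP_Vehicle2 and swapping driving and stopped sounds.
; Box overlaps detect cars ahead and flag a crash and destroy-all in GameState when hitting the player's motion controller.
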(event OnComponentBeginOverlap(Box)
  (params (OverlappedComponent :type Primitive%20Component%20Object%20Reference) (OtherActor :type Actor%20Object%20Reference) (OtherComp :type Primitive%20Component%20Object%20Reference) (OtherBodyIndex :type Integer) (bFromSweep :type Boolean) (SweepResult :type Hit%20Result%20Structure%20%28by%20ref%29))
  (bind _returnvalue (Utilities|GetClass OtherActor))
  ;[1 1 1] Responsible for checking if a car hits another car
  (if (== _returnvalue "BP_Vehicle2_C")
    (Variables|Default|SetCheckIfCarInFrontIsVehicle true)
    (else
      ;[1 1 1] Responsible for checking if a car hits a player
      (if (== _returnvalue "/Game/VirtualRealityBP/Blueprints/BP_MotionController.BP_MotionController_C")
        (bind _asgame_state_bachelor (Utilities|Casting|CastToGameState_Bachelor (Game|GetGameState))
          (:then
            (Variables|/Game/GamesBaseogState/GameState_Bachelor.GameState_Bachelor_C|SetCrashed _asgame_state_bachelor true)
            (Variables|/Game/GamesBaseogState/GameState_Bachelor.GameState_Bachelor_C|SetDestroyAllCars _asgame_state_bachelor true))
          (:CastFailed
            (Development|PrintString "Vehicle2: Destroy cars when actor hit")))
        (else
          (Variables|Default|SetCheckIfCarInFrontIsVehicle false))))))

(event OnComponentEndOverlap(Box)
  (params (OverlappedComponent :type Primitive%20Component%20Object%20Reference) (OtherActor :type Actor%20Object%20Reference) (OtherComp :type Primitive%20Component%20Object%20Reference) (OtherBodyIndex :type Integer))
  ;[1 1 1] Responsible for checking if a car hits another car
  (Variables|Default|SetCheckIfCarInFrontIsVehicle false))

(event Custom|Run_Event
  ;[1 1 1] Responsible for setting a random static mesh in list to the actor
  (bind _asgame_state_bachelor (Utilities|Casting|CastToGameState_Bachelor (Game|GetGameState))
    (:then
      (bind _returnvalue (AddComponent|AddStaticMeshComponent false))
      (Collision|SetCollisionEnabled _returnvalue "QueryAndPhysics")
      (CallFunction|SetMaterial _returnvalue (Utilities|Array|Get(acopy) (Variables|/Game/GamesBaseogState/GameState_Bachelor.GameState_Bachelor_C|GetColorsForCars _asgame_state_bachelor) (Math|Random|RandomIntegerinRange 0 (Utilities|Array|LastIndex (Variables|/Game/GamesBaseogState/GameState_Bachelor.GameState_Bachelor_C|GetColorsForCars _asgame_state_bachelor)))))
      (Components|StaticMesh|SetStaticMesh _returnvalue (Utilities|Array|Get(acopy) (Variables|/Game/GamesBaseogState/GameState_Bachelor.GameState_Bachelor_C|GetStaticMeshes _asgame_state_bachelor) (Math|Random|RandomIntegerinRange 0 (Utilities|Array|LastIndex (Variables|/Game/GamesBaseogState/GameState_Bachelor.GameState_Bachelor_C|GetStaticMeshes _asgame_state_bachelor)))))
      (Variables|Default|SetOriginalRot (Transformation|GetWorldRotation (Variables|Default|GetScene))))
    (:CastFailed
      (Development|PrintString "Cast Failed at Vehicle"))))

(event EventTick
  (params (DeltaSeconds :type Float%20%28single-precision%29))
  (bind _scene (Variables|Default|GetScene))
  (bind _scene_2 (Variables|Default|GetScene))
  (bind _scene_3 (Variables|Default|GetScene))
  (bind _scene_4 (Variables|Default|GetScene))
  (bind _scene_5 (Variables|Default|GetScene))
  (bind _caratpedestrian (Variables|Default|GetCarAtPedestrian))
  (bind _carsound (Variables|Default|GetCarSound))
  (bind _scene_6 (Variables|Default|GetScene))
  (bind _originalrot (Variables|Default|GetOriginalRot))
  (bind _returnvalue (Transformation|GetWorldLocation _scene_4))
  (bind _returnvalue_2 (Transformation|GetWorldLocation _scene_2))
  (bind _returnvalue_3 (Transformation|GetWorldRotation _scene))
  (bind (_roll _pitch _yaw) (Math|Rotator|BreakRotator _originalrot))
  (bind _returnvalue_4 (Transformation|GetWorldLocation _scene_3))
  (bind _returnvalue_5 (Transformation|GetWorldRotation _scene_6))
  (bind (_x _y _z) (Math|Vector|BreakVector _returnvalue))
  (bind (_x_2 _y_2 _z_2) (Math|Vector|BreakVector _returnvalue_2))
  (bind (_roll_2 _pitch_2 _yaw_2) (Math|Rotator|BreakRotator _returnvalue_3))
  (bind (_x_3 _y_3 _z_3) (Math|Vector|BreakVector _returnvalue_4))
  (bind (_roll_3 _pitch_3 _yaw_3) (Math|Rotator|BreakRotator _returnvalue_5))
  (Variables|Default|SetDeltaTime DeltaSeconds)
  (Utilities|FlowControl|Sequence
    (:then_0
      ;[1 1 1] Car sound
      (if (not (stale _output_get))
        (Audio|Components|Audio|Play (Variables|Default|GetCarSound) 0.0)
        (bind _output_get (Variables|Default|Setplay true))))
    (:then_1
      ;[1 1 1] Turning the car in the right turn for side 1
      (if (Variables|Default|GetTurn)
        (if (<= (- (Variables|Default|GetMoveSpeed) 399.0) 2e+02)
          _
          (else
            (Variables|Default|SetMoveSpeed (+ (- (Variables|Default|GetMoveSpeed) 399.0) 2.0))))
        (Transformation|SetWorldLocationAndRotation _scene (Math|Interpolation|VInterpTo (Transformation|GetWorldLocation _scene) (Variables|/Game/GamesBaseogState/GameState_Bachelor.GameState_Bachelor_C|GetTurns2To1 (stale Custom|Run_Event _asgame_state_bachelor)) (Variables|Default|GetDeltaTime) (- (Variables|Default|GetMoveSpeed) 399.0)) (Math|Interpolation|RInterpTo _returnvalue_3 (Math|Rotator|MakeRotator _roll_2 _pitch_2 (- _yaw_2 4.0)) (Variables|Default|GetDeltaTime) (- (Variables|Default|GetMoveSpeed) 399.0)) true false)
        (elif (Variables|Default|GetTurn2)
          (if (<= (- (Variables|Default|GetMoveSpeed) 399.0) 2e+02)
            _
            (else
              (Variables|Default|SetMoveSpeed (+ (- (Variables|Default|GetMoveSpeed) 399.0) 2.0))))
          (Transformation|SetWorldLocationAndRotation _scene_6 (Math|Interpolation|VInterpTo (Transformation|GetWorldLocation _scene_6) (Variables|/Game/GamesBaseogState/GameState_Bachelor.GameState_Bachelor_C|GetTurns2To2 (stale Custom|Run_Event _asgame_state_bachelor)) (Variables|Default|GetDeltaTime) (- (Variables|Default|GetMoveSpeed) 399.0)) (Math|Interpolation|RInterpTo _returnvalue_5 (Math|Rotator|MakeRotator _roll_3 _pitch_3 (- _yaw_3 55.0)) (Variables|Default|GetDeltaTime) (- (Variables|Default|GetMoveSpeed) 399.0)) true false)
          (elif (Variables|Default|GetTurn3)
            (if (<= (- (Variables|Default|GetMoveSpeed) 399.0) 2e+02)
              _
              (else
                (Variables|Default|SetMoveSpeed (+ (- (Variables|Default|GetMoveSpeed) 399.0) 2.0))))
            (Transformation|SetWorldLocationAndRotation _scene_5 (Math|Interpolation|VInterpTo (Transformation|GetWorldLocation _scene_5) (Variables|/Game/GamesBaseogState/GameState_Bachelor.GameState_Bachelor_C|GetTurns2To3 (stale Custom|Run_Event _asgame_state_bachelor)) (Variables|Default|GetDeltaTime) (- (Variables|Default|GetMoveSpeed) 399.0)) (Math|Rotator|MakeRotator _roll _pitch (- _yaw 9e+01)) true false)
            (else
              ;[1 1 1] The logic for if a car should stop behind another car, drive or slow down to a full stop. It also is responsible for stoping the car if it hits another car
              (if (Variables|Default|GetHaveTurned)
                ;[1 1 1] Driving in -x direction
                (if (>= (Variables|Default|GetMoveSpeed) 4e+02)
                  _
                  (else
                    (Variables|Default|SetMoveSpeed (+ (Variables|Default|GetMoveSpeed) 2.0))))
                (Transformation|SetWorldLocation _scene_4 (Math|Vector|MakeVector (+ _x (* (Variables|Default|GetMoveSpeed) (Variables|Default|GetDeltaTime))) _y _z) true false)
                (elif (Variables|Default|GetCheckIfCarInFrontIsVehicle)
                  (Utilities|FlowControl|Sequence
                    (:then_0
                      ;[1 1 1] Car sound
                      (if (not (stale _output_get_2))
                        (Audio|Components|Audio|Stop _carsound)
                        (Audio|Components|Audio|Play _caratpedestrian 0.0)
                        (bind _output_get_2 (Variables|Default|SetStop1 true))))
                    (:then_1
                      (Transformation|SetWorldLocation _scene_2 (Transformation|GetWorldLocation _scene_2) true false)))
                  (elif (Variables|Default|GetStops)
                    (Utilities|FlowControl|Sequence
                      (:then_0
                        (if (not (stale _output_get_3))
                          (Audio|Components|Audio|Stop _carsound)
                          (Audio|Components|Audio|Play _caratpedestrian 0.0)
                          (bind _output_get_3 (Variables|Default|SetStop2 true))))
                      (:then_1
                        ;[1 1 1] Responsible for slowing the car down until it stops
                        (if (<= (Variables|Default|GetMoveSpeed) 0.0)
                          _
                          (else
                            (Variables|Default|SetMoveSpeed (- (Variables|Default|GetMoveSpeed) 3.0))))
                        (Transformation|SetWorldLocation _scene_2 (Math|Vector|MakeVector _x_2 (+ _y_2 (* (Variables|Default|GetMoveSpeed) (Variables|Default|GetDeltaTime))) _z_2) true false))
                      (:then_2
                        (Variables|/Game/GamesBaseogState/GameState_Bachelor.GameState_Bachelor_C|Setcar%20stopped (stale Custom|Run_Event _asgame_state_bachelor) true)))
                    (else
                      (Utilities|FlowControl|Sequence
                        (:then_0
                          (if (not (stale _output_get_4))
                            (Audio|Components|Audio|Stop _caratpedestrian)
                            (Audio|Components|Audio|Play _carsound 0.0)
                            (bind _output_get_4 (Variables|Default|SetDrive true))))
                        (:then_1
                          ;[1 1 1] Driving in -y direction
                          (if (>= (Variables|Default|GetMoveSpeed) 4e+02)
                            _
                            (else
                              (Variables|Default|SetMoveSpeed (+ (Variables|Default|GetMoveSpeed) 1e+02))))
                          (Transformation|SetWorldLocation _scene_3 (Math|Vector|MakeVector _x_3 (+ _y_3 (* (Variables|Default|GetMoveSpeed) (Variables|Default|GetDeltaTime))) _z_3) true false))))))))))))))

(fn ConstructionScript)

(fn SetMaterial
  (params (StaticMeshComponent :type Static%20Mesh%20Component%20Object%20Reference) (Color :type Material%20Object%20Reference))
  (bind _returnvalue (Rendering|Material|CreateDynamicMaterialInstance "/Game/Models/Vehicle/M_Windows.M_Windows" :!class /Script/Engine.KismetMaterialLibrary))
  (Rendering|Material|SetMaterial StaticMeshComponent 0 _returnvalue)
  (Rendering|Material|SetMaterial StaticMeshComponent 1 Color)
  (bind _returnvalue_2 (Rendering|Material|CreateDynamicMaterialInstance "/Game/Models/Vehicle/M_Rims.M_Rims" :!class /Script/Engine.KismetMaterialLibrary))
  (Rendering|Material|SetMaterial StaticMeshComponent 2 _returnvalue_2)
  (bind _returnvalue_3 (Rendering|Material|CreateDynamicMaterialInstance "/Game/Models/Vehicle/M_FrontLights.M_FrontLights" :!class /Script/Engine.KismetMaterialLibrary))
  (Rendering|Material|SetMaterial StaticMeshComponent 3 _returnvalue_3)
  (bind _returnvalue_4 (Rendering|Material|CreateDynamicMaterialInstance "/Game/Models/Vehicle/M_Indicators.M_Indicators" :!class /Script/Engine.KismetMaterialLibrary))
  (Rendering|Material|SetMaterial StaticMeshComponent 4 _returnvalue_4)
  (bind _returnvalue_5 (Rendering|Material|CreateDynamicMaterialInstance "/Game/Models/Vehicle/M_Tires.M_Tires" :!class /Script/Engine.KismetMaterialLibrary))
  (Rendering|Material|SetMaterial StaticMeshComponent 5 _returnvalue_5)
  (return))