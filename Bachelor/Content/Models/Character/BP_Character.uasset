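; Instructor character for a pedestrian road-crossing trainer, narrating three scenario intros, demonstrating the crossing and giving spoken feedback.
; Intro events chain delayed voice cues, start cars through GameState_Bachelor, then trigger a flag-driven Tick sequence that turns, looks left-right-left, crosses and hands over to the player.
; Feedback events pick cues from GameState's looking, car-stop and light results.
; Tick also drives idle bobbing, timeline mouth scaling and crash audio.
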(event Custom|Intro_scenario_2_Event
  (bind _returnvalue (Game|GetGameState))
  ;[1 1 1] Intro scenario 2
  (Variables|Default|SetIsCharacterTalking true)
  (Audio|Components|Audio|Play (Variables|Default|Getintro_1_-_lys_Cue) 0.0)
  (Utilities|FlowControl|Delay 11.0)
  (Audio|Components|Audio|Play (Variables|Default|Getintro_2_-_lys_Cue) 0.0)
  (Utilities|FlowControl|Delay 9.0)
  (Audio|Components|Audio|Play (Variables|Default|Getintro_3_-_ys_Cue) 0.0)
  (Utilities|FlowControl|Delay 17.0)
  (bind _asgame_state_bachelor (Utilities|Casting|CastToGameState_Bachelor _returnvalue)
    (:then
      (Variables|/Game/GamesBaseogState/GameState_Bachelor.GameState_Bachelor_C|SetStartCarsLeft _asgame_state_bachelor true)
      (Utilities|FlowControl|Delay 12.0)
      (bind _asgame_state_bachelor_2 (Utilities|Casting|CastToGameState_Bachelor _returnvalue))
      (Variables|/Game/GamesBaseogState/GameState_Bachelor.GameState_Bachelor_C|SetStartCarsRight _asgame_state_bachelor_2 true)
      (Variables|Default|SetIsCharacterTalking false)
      (Variables|Default|SetCrossRoad true))
    (:CastFailed
      (Development|PrintString "Hello"))))

(event Custom|feedback_scen2_Event
  ;[1 1 1] Initialize event for scenario2/3
  (bind _asgame_state_bachelor (Utilities|Casting|CastToGameState_Bachelor (Game|GetGameState))
    (:then
      (Variables|Default|SetLocalCarStopVariable (Variables|/Game/GamesBaseogState/GameState_Bachelor.GameState_Bachelor_C|Getcar%20stopped _asgame_state_bachelor))
      ;[1 1 1] LRL feedback
      (if (Variables|/Game/GamesBaseogState/GameState_Bachelor.GameState_Bachelor_C|GetLRL _asgame_state_bachelor)
        (Variables|Default|SetIsCharacterTalking true)
        (Audio|Components|Audio|Play (Variables|Default|GetLRL_alt_rett_Cue) 0.0)
        (Utilities|FlowControl|Delay 1e+01)
        (else
          (Variables|Default|SetIsCharacterTalking true)
          (if (Variables|/Game/GamesBaseogState/GameState_Bachelor.GameState_Bachelor_C|GetLookRight _asgame_state_bachelor)
            (Audio|Components|Audio|Play (Variables|Default|GetLR_en_feil_Cue) 0.0)
            (Utilities|FlowControl|Delay 18.5)
            (elif (Variables|/Game/GamesBaseogState/GameState_Bachelor.GameState_Bachelor_C|GetLookLeftFirst _asgame_state_bachelor)
              (Audio|Components|Audio|Play (Variables|Default|GetL_to_feil_Cue) 0.0)
              (Utilities|FlowControl|Delay 18.5)
              (else
                (Audio|Components|Audio|Play (Variables|Default|Getalt_feil_i_LRL_Cue) 0.0)
                (Utilities|FlowControl|Delay 6.0))))))
      ;[1 1 1] Did the car stop?
      (if (Variables|/Game/GamesBaseogState/GameState_Bachelor.GameState_Bachelor_C|GetCarStopMedianSave%20 _asgame_state_bachelor)
        (Audio|Components|Audio|Play (Variables|Default|Getbil_stoppet_riktig_Cue) 0.0)
        (Utilities|FlowControl|Delay 4.5)
        (else
          (Audio|Components|Audio|Play (Variables|Default|Getbilene_sto_ikke_i_ro) 0.0)
          (Utilities|FlowControl|Delay 6.0)))
      ;[1 1 1] Feedback regarding lights
      (if (Variables|/Game/GamesBaseogState/GameState_Bachelor.GameState_Bachelor_C|GetLightsMedianSave _asgame_state_bachelor)
        (Audio|Components|Audio|Play (Variables|Default|Getredlight_Cue) 0.0)
        (else
          (Audio|Components|Audio|Play (Variables|Default|Getgreenlight_Cue) 0.0)))
      (Variables|Default|SetIsCharacterTalking false))
    (:CastFailed
      (Development|PrintString "Cast to gamestate failed at feedback portion of Character_blueprint"))))

(event Custom|Intro_scenario_1_Event
  ;[1 1 1] Intro scenario 1
  (Variables|Default|SetIsCharacterTalking true)
  (Audio|Components|Audio|Play (Variables|Default|Getintro_2_Cue) 0.0)
  (Utilities|FlowControl|Delay 6.0)
  (Audio|Components|Audio|Play (Variables|Default|Getintro3_Cue) 0.0)
  (Utilities|FlowControl|Delay 4.0)
  (Audio|Components|Audio|Play (Variables|Default|Getintro4_forttau_Cue) 0.0)
  (Utilities|FlowControl|Delay 1e+01)
  (Audio|Components|Audio|Play (Variables|Default|Getintro_5_lrl_hvordan_RETT_Cue) 0.0)
  (Utilities|FlowControl|Delay 17.0)
  (Audio|Components|Audio|Play (Variables|Default|GetLRL_hvorfor_Cue) 0.0)
  (Utilities|FlowControl|Delay 4.0)
  (Audio|Components|Audio|Play (Variables|Default|Getsiste_gjennomgang_Cue) 0.0)
  (Utilities|FlowControl|Delay 28.0)
  (Audio|Components|Audio|Play (Variables|Default|Getdemonstrasjon_Cue) 0.0)
  (bind _asgame_state_bachelor (Utilities|Casting|CastToGameState_Bachelor (Game|GetGameState)))
  (Variables|/Game/GamesBaseogState/GameState_Bachelor.GameState_Bachelor_C|SetStartCarsLeft _asgame_state_bachelor true)
  (Utilities|FlowControl|Delay 12.0)
  (bind _asgame_state_bachelor_2 (Utilities|Casting|CastToGameState_Bachelor (Game|GetGameState)))
  (Variables|/Game/GamesBaseogState/GameState_Bachelor.GameState_Bachelor_C|SetStartCarsRight _asgame_state_bachelor_2 true)
  (Variables|Default|SetIsCharacterTalking false)
  (Variables|Default|SetCrossRoad true))

(event Custom|feedback_Event
  ;[1 1 1] Initialize event for scenario 1
  (bind _asgame_state_bachelor (Utilities|Casting|CastToGameState_Bachelor (Game|GetGameState))
    (:then
      ;[1 1 1] LRL feedback
      (if (Variables|/Game/GamesBaseogState/GameState_Bachelor.GameState_Bachelor_C|GetLRL _asgame_state_bachelor)
        (Variables|Default|SetIsCharacterTalking true)
        (Audio|Components|Audio|Play (Variables|Default|GetLRL_alt_rett_Cue) 0.0)
        (Utilities|FlowControl|Delay 1e+01)
        (else
          (Variables|Default|SetIsCharacterTalking true)
          (if (Variables|/Game/GamesBaseogState/GameState_Bachelor.GameState_Bachelor_C|GetLookRight _asgame_state_bachelor)
            (Audio|Components|Audio|Play (Variables|Default|GetLR_en_feil_Cue) 0.0)
            (Utilities|FlowControl|Delay 18.5)
            (elif (Variables|/Game/GamesBaseogState/GameState_Bachelor.GameState_Bachelor_C|GetLookLeftFirst _asgame_state_bachelor)
              (Audio|Components|Audio|Play (Variables|Default|GetL_to_feil_Cue) 0.0)
              (Utilities|FlowControl|Delay 18.5)
              (else
                (Audio|Components|Audio|Play (Variables|Default|Getalt_feil_i_LRL_Cue) 0.0)
                (Utilities|FlowControl|Delay 6.0))))))
      ;[1 1 1] Did the car stop?
      (if (Variables|/Game/GamesBaseogState/GameState_Bachelor.GameState_Bachelor_C|Getcar%20stopped _asgame_state_bachelor)
        (Audio|Components|Audio|Play (Variables|Default|Getbil_stoppet_riktig_Cue) 0.0)
        (Utilities|FlowControl|Delay 4.5)
        (else
          (Audio|Components|Audio|Play (Variables|Default|GetBil_stoppet_Cue) 0.0)
          (Utilities|FlowControl|Delay 1e+01)))
      (Variables|Default|SetIsCharacterTalking false))
    (:CastFailed
      (Development|PrintString "Cast to gamestate failed at feedback portion of Character_blueprint"))))

(event Custom|Intro_scenario_3_Event
  ;[1 1 1] Intro scenario 3
  (bind _asgame_state_bachelor (Utilities|Casting|CastToGameState_Bachelor (Game|GetGameState))
    (:then
      (Variables|Default|SetIsCharacterTalking true)
      (Audio|Components|Audio|Play (Variables|Default|GetSCENARIO_3_INTRO) 0.0)
      (Utilities|FlowControl|Delay 1e+01)
      (Variables|/Game/GamesBaseogState/GameState_Bachelor.GameState_Bachelor_C|SetStartCarsLeft _asgame_state_bachelor true)
      (Utilities|FlowControl|Delay 11.0)
      (Variables|/Game/GamesBaseogState/GameState_Bachelor.GameState_Bachelor_C|SetStartCarsRight _asgame_state_bachelor true)
      (Variables|Default|SetIsCharacterTalking false)
      (Variables|Default|SetCrossRoad true))
    (:CastFailed
      (Development|PrintString "Cast to gamestate failed at intro to scenario 3 CharacterBP"))))

(event EventTick
  (params (DeltaSeconds :type Float%20%28single-precision%29))
  (bind _returnvalue (Transformation|GetActorRotation))
  (bind _returnvalue_2 (Transformation|GetActorLocation))
  (bind _returnvalue_3 (Transformation|GetActorRotation))
  (bind _returnvalue_4 (Transformation|GetActorRotation))
  (bind _returnvalue_5 (Transformation|GetActorLocation))
  (bind _returnvalue_6 (Transformation|GetActorRotation))
  (bind _returnvalue_7 (Transformation|GetActorRotation))
  (bind _returnvalue_8 (Transformation|GetActorRotation))
  (bind _mouth (Variables|Default|GetMouth))
  (bind (_roll _pitch _yaw) (Math|Rotator|BreakRotator _returnvalue))
  (bind (_x _y _z) (Math|Vector|BreakVector _returnvalue_2))
  (bind (_roll_2 _pitch_2 _yaw_2) (Math|Rotator|BreakRotator _returnvalue_3))
  (bind (_roll_3 _pitch_3 _yaw_3) (Math|Rotator|BreakRotator _returnvalue_4))
  (bind (_x_2 _y_2 _z_2) (Math|Vector|BreakVector _returnvalue_5))
  (bind (_roll_4 _pitch_4 _yaw_4) (Math|Rotator|BreakRotator _returnvalue_6))
  (bind (_roll_5 _pitch_5 _yaw_5) (Math|Rotator|BreakRotator _returnvalue_7))
  (bind (_roll_6 _pitch_6 _yaw_6) (Math|Rotator|BreakRotator _returnvalue_8))
  (bind _returnvalue_9 (Transformation|GetWorldScale _mouth))
  (bind (_x_3 _y_3) (Math|Vector|BreakVector _returnvalue_9))
  ;[1 1 1] Event tick and sequence
  (Variables|Default|SetDeltaTime DeltaSeconds)
  (Utilities|FlowControl|Sequence
    (:then_0
      ;[1 1 1] Set location
      (if (Variables|Default|GetSetLocation)
        ;[1 1 1] Comment
        (if (Variables|Default|GetCrossRoad)
          (Utilities|FlowControl|Sequence
            (:then_0
              ;[1 1 1] Step 1 done?
              (if (Variables|Default|GetStep1)
                ;[1 1 1] Set location
                (if (Variables|Default|GetNewLocation1)
                  ;[1 1 1] Step 2 done?
                  (if (Variables|Default|GetStep2)
                    ;[1 1 1] Set rotation
                    (if (Variables|Default|GetNewRotation)
                      ;[1 1 1] Step 3 done?
                      (if (Variables|Default|GetPart3)
                        ;[1 1 1] Set rotation
                        (if (Variables|Default|GetNewRotation2)
                          ;[1 1 1] Step 4 done?
                          (if (Variables|Default|GetPart4)
                            ;[1 1 1] Set rotation
                            (if (Variables|Default|GetNewRotation3)
                              ;[1 1 1] Step 5 done?
                              (if (Variables|Default|GetPart5)
                                ;[1 1 1] Set rotation
                                (if (Variables|Default|GetNewRotation4)
                                  ;[1 1 1] Step 6 done?
                                  (if (Variables|Default|GetStap6)
                                    ;[1 1 1] Set location
                                    (if (Variables|Default|GetNewLocation2)
                                      ;[1 1 1] Step 7 done?
                                      (if (Variables|Default|GetStep7)
                                        ;[1 1 1] Set rotation
                                        (if (Variables|Default|GetNewRotation5)
                                          ;[1 1 1] Step 8 done?
                                          (if (not (Variables|Default|GetStep8))
                                            ;[1 1 1] Character crosses the road 8: Rotates towards the player
                                            (if (>= _yaw_5 (- (.Yaw (Math|Rotator|BreakRotator (Variables|Default|GetCharacterRotation))) 2.4e+02))
                                              (Transformation|SetActorRotation (Math|Interpolation|RInterpTo _returnvalue_7 (Math|Rotator|MakeRotator _roll_5 _pitch_5 (- _yaw_5 (* (Variables|Default|GetDeltaTime) 5e+03))) (Variables|Default|GetDeltaTime) 1.0))
                                              (else
                                                (Variables|Default|SetStep8 true)
                                                ;[1 1 1] Move up and down = true
                                                (Variables|Default|SetCrossRoad false)
                                                (Variables|Default|SetSetLocation false)
                                                ;[1 1 1] Plays instruction
                                                (Audio|Components|Audio|Play (Variables|Default|Getyour_turn_to_try) 0.0)
                                                (Variables|Default|SetIsCharacterTalking true)
                                                (Utilities|FlowControl|Delay 3.0)
                                                (Variables|Default|SetIsCharacterTalking false)
                                                (bind _asgame_state_bachelor (Utilities|Casting|CastToGameState_Bachelor (Game|GetGameState)))
                                                (Variables|/Game/GamesBaseogState/GameState_Bachelor.GameState_Bachelor_C|SetIntroFinished _asgame_state_bachelor true))))
                                          (else
                                            (Utilities|FlowControl|Delay 0.2)
                                            (Variables|Default|SetCharacterRotation (Transformation|GetActorRotation))
                                            (Variables|Default|SetNewRotation5 true)))
                                        (else
                                          ;[1 1 1] Character crosses the road 7: Crosses the road
                                          (if (>= _x (- (.X (Math|Vector|BreakVector (Variables|Default|GetCharacterLocation))) 5.5e+02))
                                            (Transformation|SetActorLocation (Math|Interpolation|VInterpTo _returnvalue_2 (Math|Vector|MakeVector (- _x (* (Variables|Default|GetDeltaTime) (Variables|Default|GetWalkSpeed))) _y _z) (Variables|Default|GetDeltaTime) 0.5) false false)
                                            (else
                                              (Variables|Default|SetStep7 true)))))
                                      (else
                                        (Utilities|FlowControl|Delay 0.2)
                                        (Variables|Default|SetCharacterLocation (Transformation|GetActorLocation))
                                        (Variables|Default|SetNewLocation2 true)))
                                    (else
                                      ;[1 1 1] Character crosses the road 6: Character rotates towards the road
                                      (if (>= _yaw_2 (+ (.Yaw (Math|Rotator|BreakRotator (Variables|Default|GetCharacterRotation))) 6e+01))
                                        (Variables|Default|SetStap6 true)
                                        (else
                                          (Transformation|SetActorRotation (Math|Interpolation|RInterpTo _returnvalue_3 (Math|Rotator|MakeRotator _roll_2 _pitch_2 (+ _yaw_2 (* (Variables|Default|GetDeltaTime) 5e+03))) (Variables|Default|GetDeltaTime) 1.0))))))
                                  (else
                                    (Utilities|FlowControl|Delay 0.2)
                                    (Variables|Default|SetCharacterRotation (Transformation|GetActorRotation))
                                    (Variables|Default|SetNewRotation4 true)))
                                (else
                                  ;[1 1 1] Character crosses the road 5: Character checks left 2
                                  (if (>= _yaw_4 (- (.Yaw (Math|Rotator|BreakRotator (Variables|Default|GetCharacterRotation))) 1.3e+02))
                                    (Transformation|SetActorRotation (Math|Interpolation|RInterpTo _returnvalue_6 (Math|Rotator|MakeRotator _roll_4 _pitch_4 (- _yaw_4 (* (Variables|Default|GetDeltaTime) 5e+03))) (Variables|Default|GetDeltaTime) 1.0))
                                    (else
                                      (Variables|Default|SetPart5 true)))))
                              (else
                                (Utilities|FlowControl|Delay 0.2)
                                (Variables|Default|SetCharacterRotation (Transformation|GetActorRotation))
                                (Variables|Default|SetNewRotation3 true)))
                            (else
                              ;[1 1 1] Character crosses the road 4: Character checks right
                              (if (>= _yaw_6 (+ (.Yaw (Math|Rotator|BreakRotator (Variables|Default|GetCharacterRotation))) 1.5e+02))
                                (Variables|Default|SetPart4 true)
                                (else
                                  (Transformation|SetActorRotation (Math|Interpolation|RInterpTo _returnvalue_8 (Math|Rotator|MakeRotator _roll_6 _pitch_6 (+ _yaw_6 (* (Variables|Default|GetDeltaTime) 5e+03))) (Variables|Default|GetDeltaTime) 1.0))))))
                          (else
                            (Utilities|FlowControl|Delay 0.2)
                            (Variables|Default|SetCharacterRotation (Transformation|GetActorRotation))
                            (Variables|Default|SetNewRotation2 true)))
                        (else
                          ;[1 1 1] Character crosses the road 3; Character checks left 1
                          (if (>= _yaw_3 (- (.Yaw (Math|Rotator|BreakRotator (Variables|Default|GetCharacterRotation))) 8e+01))
                            (Transformation|SetActorRotation (Math|Interpolation|RInterpTo _returnvalue_4 (Math|Rotator|MakeRotator _roll_3 _pitch_3 (- _yaw_3 (* (Variables|Default|GetDeltaTime) 5e+03))) (Variables|Default|GetDeltaTime) 1.0))
                            (else
                              (Variables|Default|SetPart3 true)))))
                      (else
                        (Variables|Default|SetCharacterRotation (Transformation|GetActorRotation))
                        (Variables|Default|SetNewRotation true)))
                    (else
                      ;[1 1 1] Character crosses the road 2: Walks over to the road
                      (if (>= _x_2 (- (.X (Math|Vector|BreakVector (Variables|Default|GetCharacterLocation))) 4e+01))
                        (Transformation|SetActorLocation (Math|Interpolation|VInterpTo _returnvalue_5 (Math|Vector|MakeVector (- _x_2 (* (Variables|Default|GetDeltaTime) (Variables|Default|GetWalkSpeed))) _y_2 _z_2) (Variables|Default|GetDeltaTime) 0.5) false false)
                        (else
                          (Variables|Default|SetStep2 true)))))
                  (else
                    (Variables|Default|SetCharacterLocation (Transformation|GetActorLocation))
                    (Variables|Default|SetNewLocation1 true)))
                (else
                  ;[1 1 1] Character crosses the road 1: Rotates the character to the left.
                  (if (>= _yaw (- (.Yaw (Math|Rotator|BreakRotator (Variables|Default|GetCharacterRotation))) 6e+01))
                    (Transformation|SetActorRotation (Math|Interpolation|RInterpTo _returnvalue (Math|Rotator|MakeRotator _roll _pitch (- _yaw (* (Variables|Default|GetDeltaTime) 3.5e+03))) (Variables|Default|GetDeltaTime) 1.0))
                    (else
                      (Variables|Default|SetStep1 true))))))
            (:then_1
              ;[1 1 1] Moved the character up and down
              (bind _newtrack_0 (Timeline|TimelineCharacter Stop)
                (:Update
                  (Transformation|SetActorLocation (Math|Vector|MakeVector (.X (Math|Vector|BreakVector (Variables|Default|GetCharacterLocation))) (.Y (Math|Vector|BreakVector (Variables|Default|GetCharacterLocation))) (+ (.Z (Math|Vector|BreakVector (Variables|Default|GetCharacterLocation))) _newtrack_0)) false false)))))
          (else
            (Timeline|TimelineCharacter Play)))
        (else
          (Variables|Default|SetCharacterLocation (Transformation|GetActorLocation))
          (Variables|Default|SetSetLocation true))))
    (:then_1
      ;[1 1 1] Boolean: Is the character talking?
      (if (Variables|Default|GetIsCharacterTalking)
        ;[1 1 1] Scales the mouth when the character is talking
        (bind _newtrack_2 (Timeline|TimelineMouth Play)
          (:Update
            (Transformation|SetWorldScale3D (Variables|Default|GetMouth) (Math|Vector|MakeVector _x_3 _y_3 _newtrack_2))))
        (else
          (Timeline|TimelineMouth Stop))))
    (:then_2
      ;[1 1 1] Crash feedback
      (if (Variables|/Game/GamesBaseogState/GameState_Bachelor.GameState_Bachelor_C|GetCrashed (stale EventBeginPlay _asgame_state_bachelor))
        (Audio|Components|Audio|Play (Variables|Default|GetS_accident) 0.0)
        (Variables|/Game/GamesBaseogState/GameState_Bachelor.GameState_Bachelor_C|SetCrashed (stale EventBeginPlay _asgame_state_bachelor) false)))))

(event EventBeginPlay
  ;[1 1 1] Event beginplay and sequence
  (bind _asgame_state_bachelor (Utilities|Casting|CastToGameState_Bachelor (Game|GetGameState)))
  (Variables|Default|SetCharacterLocation (Transformation|GetActorLocation))
  ;[1 1 1] Character crosses the road 1: Rotates the character to the left.
  (Variables|Default|SetCharacterRotation (Transformation|GetActorRotation)))

(fn ConstructionScript)