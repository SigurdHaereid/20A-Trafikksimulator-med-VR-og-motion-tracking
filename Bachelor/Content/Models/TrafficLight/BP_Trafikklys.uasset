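; Traffic light actor that runs a timed signal cycle for cars and pedestrians.
; BeginPlay starts with car red and pedestrian green for a long initial hold, then loops a Delay chain through all-red, yellow, car green and pedestrian green phases.
; Each phase sets light component intensities and swaps lit/dark materials on mesh slots.
; It publishes RedLightCar and RedLightPedestrian flags to GameState_Bachelor, printing an error if a cast fails.
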(event EventBeginPlay
  (bind _staticmeshcomponent (Variables|Debug|GetStaticMeshComponent))
  (bind _staticmeshcomponent_2 (Variables|Debug|GetStaticMeshComponent))
  ;[1 1 1] light off
  (Rendering|Components|Light|SetIntensity (Variables|Default|GetYellowCar) 0.0)
  ;[1 1 1] Red light on for cars
  (Rendering|Components|Light|SetIntensity (Variables|Default|GetRedCar) 2e+03)
  (Rendering|Material|SetMaterial (Variables|Debug|GetStaticMeshComponent) 1 "/Game/Farger/M_LightRed.M_LightRed")
  ;[1 1 1] Green light on for pedestrians
  (Rendering|Components|Light|SetIntensity (Variables|Default|GetGreenPedestrian) 8e+02)
  (Rendering|Material|SetMaterial (Variables|Debug|GetStaticMeshComponent) 3 "/Game/Farger/M_LightGreen.M_LightGreen")
  (Utilities|FlowControl|Delay 65.0)
  (Rendering|Material|SetMaterial (Variables|Debug|GetStaticMeshComponent) 3 "/Game/Farger/M_DarkGreen.M_DarkGreen")
  (Rendering|Components|Light|SetIntensity (Variables|Default|GetYellowCar) 0.0)
  ;[1 1 1] Red light on for cars and pedestrians
  (Rendering|Components|Light|SetIntensity (Variables|Default|GetRedPedestrian) 2e+03 :!label _label)
  (bind _asgame_state_bachelor (Utilities|Casting|CastToGameState_Bachelor (Game|GetGameState))
    (:then
      (Variables|/Game/GamesBaseogState/GameState_Bachelor.GameState_Bachelor_C|SetRedLightCar _asgame_state_bachelor true)
      (Variables|/Game/GamesBaseogState/GameState_Bachelor.GameState_Bachelor_C|SetRedLightPedestrian _asgame_state_bachelor true)
      (Rendering|Material|SetMaterial _staticmeshcomponent 1 "/Game/Farger/M_LightRed.M_LightRed")
      (Rendering|Material|SetMaterial _staticmeshcomponent 2 "/Game/Farger/M_LightRed.M_LightRed")
      (Utilities|FlowControl|Delay 2.0)
      ;[1 1 1] Yellow lignt on
      (Rendering|Components|Light|SetIntensity (Variables|Default|GetYellowCar) 2e+03)
      (Rendering|Material|SetMaterial (Variables|Debug|GetStaticMeshComponent) 4 "/Game/Farger/M_LightYellow.M_LightYellow")
      (Utilities|FlowControl|Delay 2.0)
      ;[1 1 1] Yellow and red light off
      (Rendering|Components|Light|SetIntensity (Variables|Default|GetYellowCar) 0.0)
      (bind _asgame_state_bachelor_2 (Utilities|Casting|CastToGameState_Bachelor (Game|GetGameState))
        (:then
          (Variables|/Game/GamesBaseogState/GameState_Bachelor.GameState_Bachelor_C|SetRedLightCar _asgame_state_bachelor_2 false)
          (Rendering|Material|SetMaterial _staticmeshcomponent_2 4 "/Game/Farger/M_DarkYellow.M_DarkYellow")
          (Rendering|Material|SetMaterial _staticmeshcomponent_2 1 "/Game/Farger/M_DarkRed.M_DarkRed")
          ;[1 1 1] Green light on for cars
          (Rendering|Components|Light|SetIntensity (Variables|Default|GetGreenCar) 8e+02)
          (Rendering|Material|SetMaterial (Variables|Debug|GetStaticMeshComponent) 5 "/Game/Farger/M_LightGreen.M_LightGreen")
          (Utilities|FlowControl|Delay 1e+01)
          ;[1 1 1] Green light off for cars
          (Rendering|Components|Light|SetIntensity (Variables|Default|GetGreenCar) 0.0)
          (Rendering|Material|SetMaterial (Variables|Debug|GetStaticMeshComponent) 5 "/Game/Farger/M_DarkGreen.M_DarkGreen")
          ;[1 1 1] Yellow light on
          (Rendering|Components|Light|SetIntensity (Variables|Default|GetYellowCar) 2e+03)
          (Rendering|Material|SetMaterial (Variables|Debug|GetStaticMeshComponent) 4 "/Game/Farger/M_LightYellow.M_LightYellow")
          (Utilities|FlowControl|Delay 2.0)
          ;[1 1 1] Yellow light off
          (Rendering|Components|Light|SetIntensity (Variables|Default|GetYellowCar) 0.0)
          (Rendering|Material|SetMaterial (Variables|Debug|GetStaticMeshComponent) 4 "/Game/Farger/M_DarkYellow.M_DarkYellow")
          ;[1 1 1] Red light on for cars
          (Rendering|Components|Light|SetIntensity (Variables|Default|GetRedCar) 2e+03)
          (bind _asgame_state_bachelor_3 (Utilities|Casting|CastToGameState_Bachelor (Game|GetGameState))
            (:then
              (Variables|/Game/GamesBaseogState/GameState_Bachelor.GameState_Bachelor_C|SetRedLightCar _asgame_state_bachelor_3 true)
              (Rendering|Material|SetMaterial (Variables|Debug|GetStaticMeshComponent) 1 "/Game/Farger/M_LightRed.M_LightRed")
              (Utilities|FlowControl|Delay 3.0)
              ;[1 1 1] Red light off for pedestrians
              (Rendering|Components|Light|SetIntensity (Variables|Default|GetRedPedestrian) 0.0)
              (bind _asgame_state_bachelor_4 (Utilities|Casting|CastToGameState_Bachelor (Game|GetGameState))
                (:then
                  (Variables|/Game/GamesBaseogState/GameState_Bachelor.GameState_Bachelor_C|SetRedLightPedestrian _asgame_state_bachelor_4 false)
                  (Rendering|Material|SetMaterial (Variables|Debug|GetStaticMeshComponent) 2 "/Game/Farger/M_DarkRed.M_DarkRed")
                  ;[1 1 1] Green light on for pedestrians
                  (Rendering|Components|Light|SetIntensity (Variables|Default|GetGreenPedestrian) 8e+02)
                  (Rendering|Material|SetMaterial (Variables|Debug|GetStaticMeshComponent) 3 "/Game/Farger/M_LightGreen.M_LightGreen")
                  (Utilities|FlowControl|Delay 15.0)
                  ;[1 1 1] Green light off for pedestrians
                  (Rendering|Components|Light|SetIntensity (Variables|Default|GetGreenPedestrian) 0.0)
                  (Rendering|Material|SetMaterial (Variables|Debug|GetStaticMeshComponent) 3 "/Game/Farger/M_DarkGreen.M_DarkGreen")
                  ;[1 1 1] Red light on for pedestrians
                  (Rendering|Components|Light|SetIntensity (Variables|Default|GetRedPedestrian) 2e+03)
                  (Rendering|Material|SetMaterial (Variables|Debug|GetStaticMeshComponent) 2 "/Game/Farger/M_LightRed.M_LightRed")
                  (bind _asgame_state_bachelor_5 (Utilities|Casting|CastToGameState_Bachelor (Game|GetGameState))
                    (:then
                      (Variables|/Game/GamesBaseogState/GameState_Bachelor.GameState_Bachelor_C|SetRedLightPedestrian _asgame_state_bachelor_5 true)
                      (Utilities|FlowControl|Delay 3.0)
                      (goto _label))
                    (:CastFailed
                      (Development|PrintString "Cast to gamestate failed at Trafikklys_Blueprint \"Red light on for pedestrians\""))))
                (:CastFailed
                  (Development|PrintString "Cast to gamestate failed at Trafikklys_Blueprint \"Red light off for pedestrians\""))))
            (:CastFailed
              (Development|PrintString "Cast to gamestate failed at Trafikklys_Blueprint \"Red light on for cars\""))))
        (:CastFailed
          (Development|PrintString "Cast to gamestate failed at Trafikklys_Blueprint \"Red light and yellow light off\""))))
    (:CastFailed
      (Development|PrintString "Cast to gamestate failed at Trafikklys_Blueprint \"Red light on for cars and pedestrians\""))))

(fn ConstructionScript)